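; Game instance that holds persistent player progression (high score, coins, upgrade levels and prices, gun selection) and handles menu, shop and level flow.
; Init loads the save slot; EndGame keeps the best score, banks coins, saves and returns to the main menu.
; Menu and shop widgets are created lazily and reused with UI-only input.
; GetEquptedGun returns the selected gun; gun infos are saved but LoadFromFile never restores them.
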(event `ShowMainMenu`
  (bind _returnvalue (`GameplayStatics.GetPlayerController` 0))
  (`/Engine/EditorBlueprintResources/StandardMacros.IsValid` (`self.MenuUMG`)
    (:`Is Valid`
      _)
    (:`Is Not Valid`
      (bind _returnvalue_2 (`|CreateWidget` "/Game/Blueprints/UMG/StartMenuUMG.StartMenuUMG_C" _returnvalue))
      (set `self.MenuUMG` _returnvalue_2)))
  (`UserWidget.AddToViewport` (`self.MenuUMG`) 0)
  (set `PlayerController.bShowMouseCursor` true _returnvalue)
  (`WidgetBlueprintLibrary.SetInputMode_UIOnlyEx` _returnvalue (`self.MenuUMG`) "LockInFullscreen"))

(event `On Game Start`
  (`WidgetBlueprintLibrary.SetInputMode_GameOnly` (`GameplayStatics.GetPlayerController` 0))
  (`GameplayStatics.OpenLevel` "G_Map"))

(event `self.ReceiveInit`
  (`self.LoadFromFile`))

(event `OnShopOpened`
  (bind _returnvalue (`GameplayStatics.GetPlayerController` 0))
  (`Widget.RemoveFromParent` (`self.MenuUMG`))
  (`/Engine/EditorBlueprintResources/StandardMacros.IsValid` (`self.ShopUMG`)
    (:`Is Valid`
      _)
    (:`Is Not Valid`
      (bind _returnvalue_2 (`|CreateWidget` "/Game/Blueprints/UMG/ShopUMG.ShopUMG_C" _returnvalue))
      (bind _output_get (set `self.ShopUMG` _returnvalue_2))))
  (`UserWidget.AddToViewport` _output_get 0)
  (set `PlayerController.bShowMouseCursor` true _returnvalue)
  (`WidgetBlueprintLibrary.SetInputMode_UIOnlyEx` _returnvalue (`self.ShopUMG`) "LockInFullscreen"))

(fn `BackToMenu`
  (params (UMG :type "UserWidget Object Reference"))
  (bind _returnvalue (`GameplayStatics.GetPlayerController` 0))
  (`Widget.RemoveFromParent` UMG)
  (`UserWidget.AddToViewport` (`self.MenuUMG`) 0)
  (set `PlayerController.bShowMouseCursor` true _returnvalue)
  (`WidgetBlueprintLibrary.SetInputMode_UIOnlyEx` _returnvalue (`self.MenuUMG`) "LockInFullscreen"))

(fn `EndGame`
  (params (GameMode :type "/Game/Blueprints/GameModes/MyShooterGameModeBase Object Reference"))
  (bind _returnvalue (`ShooterGameModeBase.GetScore` GameMode))
  (if (> _returnvalue (`self.Score`))
    (set `self.Score` _returnvalue))
  (bind _returnvalue_2 (`ShooterGameModeBase.GetCoins` GameMode))
  (set `self.PlayerCoins` (+ (`self.PlayerCoins`) _returnvalue_2))
  (`self.SaveToFile`)
  (`GameplayStatics.OpenLevel` "MainMenu")
  (`self.ShowMainMenu`))

(fn `GetEquptedGun`
  (returns (GunTypeInfo :type "/Game/Blueprints/Sructure/ShootTypeInfo Structure") (GunType :type "/Game/Blueprints/Enums/GunTypeEnum Enum"))
  (locals (GunTypeVariable :type "/Game/Blueprints/Enums/GunTypeEnum Enum" :default "NewEnumerator0"))
  (bind _shoottypeinfos (`self.ShootTypeInfos`))
  (for (_array_element _array_index) _shoottypeinfos
    (if (`.IsSelected_27_F5D06D5243134D29700AE987B04C5E03` (break `/Game/Blueprints/Sructure/ShootingInfoStructure` _array_element))
      (break)))
  (switch `int` _array_index
    (:`0`
      (set `local.GunTypeVariable` "NewEnumerator0"))
    (:`1`
      (set `local.GunTypeVariable` "NewEnumerator1"))
    (:`2`
      (set `local.GunTypeVariable` "NewEnumerator2")))
  (bind _output_shootinginfo (break `/Game/Blueprints/Sructure/ShootingInfoStructure` (`|GetArrayItem` _shoottypeinfos _array_index)))
  (return _output_shootinginfo (`local.GunTypeVariable`)))

(fn `LoadFromFile`
  (bind _saveslotname (`self.SaveSlotName`))
  (bind _returnvalue (`GameplayStatics.DoesSaveGameExist` _saveslotname))
  (if _returnvalue
    (bind _returnvalue_2 (`GameplayStatics.LoadGameFromSlot` _saveslotname))
    (bind _assave_game_bp (cast `/Game/Blueprints/SaveGame/SaveGameBP` _returnvalue_2))
    (bind _output_get (set `self.SaveGameObject` _assave_game_bp))
    (set `self.Score` (`/Game/Blueprints/SaveGame/SaveGameBP.Score` _output_get))
    (set `self.PlayerCoins` (`/Game/Blueprints/SaveGame/SaveGameBP.Coins` _output_get))
    (set `self.CurrentHealthLvl` (`/Game/Blueprints/SaveGame/SaveGameBP.CurrentHealthLvl` _output_get))
    (set `self.CurrentSpeedLvl` (`/Game/Blueprints/SaveGame/SaveGameBP.CurrentSpeedLvl` _output_get))
    (set `self.CurrentCoinLvl` (`/Game/Blueprints/SaveGame/SaveGameBP.CurrentCoinLvl` _output_get))
    (set `self.HealthLvlChange` (`/Game/Blueprints/SaveGame/SaveGameBP.HealthLvlChange` _output_get))
    (set `self.SpeedLvlChange` (`/Game/Blueprints/SaveGame/SaveGameBP.SpeedLvlChange` _output_get))
    (set `self.CoinLvlChange` (`/Game/Blueprints/SaveGame/SaveGameBP.CoinLvlChange` _output_get))
    (set `self.HealthUpPrice` (`/Game/Blueprints/SaveGame/SaveGameBP.HealthUpPrice` _output_get))
    (set `self.SpeedUpPrice` (`/Game/Blueprints/SaveGame/SaveGameBP.SpeedUpPrice` _output_get))
    (set `self.CoinsUpPrice` (`/Game/Blueprints/SaveGame/SaveGameBP.CoinsUpPrice` _output_get))
    (set `self.PlayerAddedHealth` (`/Game/Blueprints/SaveGame/SaveGameBP.PlayerAddedHealth` _output_get))
    (set `self.PlayerSpeedMultiplayer` (`/Game/Blueprints/SaveGame/SaveGameBP.PlayerSpeedMultiplayer` _output_get))
    (set `self.AddedCoinsPerCoinBonus` (`/Game/Blueprints/SaveGame/SaveGameBP.AddedCoinsPerCoinBonus` _output_get))))

(fn `SaveToFile`
  (if (not (`KismetSystemLibrary.IsValid` (`self.SaveGameObject`)))
    (bind _returnvalue (`GameplayStatics.CreateSaveGameObject` "/Game/Blueprints/SaveGame/SaveGameBP.SaveGameBP_C"))
    (bind _output_get (set `self.SaveGameObject` _returnvalue)))
  (set `/Game/Blueprints/SaveGame/SaveGameBP.Score` (`self.Score`) _output_get)
  (set `/Game/Blueprints/SaveGame/SaveGameBP.Coins` (`self.PlayerCoins`) _output_get)
  (set `/Game/Blueprints/SaveGame/SaveGameBP.CurrentHealthLvl` (`self.CurrentHealthLvl`) _output_get)
  (set `/Game/Blueprints/SaveGame/SaveGameBP.CurrentSpeedLvl` (`self.CurrentSpeedLvl`) _output_get)
  (set `/Game/Blueprints/SaveGame/SaveGameBP.CurrentCoinLvl` (`self.CurrentCoinLvl`) _output_get)
  (set `/Game/Blueprints/SaveGame/SaveGameBP.HealthUpPrice` (`self.HealthUpPrice`) _output_get)
  (set `/Game/Blueprints/SaveGame/SaveGameBP.SpeedUpPrice` (`self.SpeedUpPrice`) _output_get)
  (set `/Game/Blueprints/SaveGame/SaveGameBP.CoinsUpPrice` (`self.CoinsUpPrice`) _output_get)
  (set `/Game/Blueprints/SaveGame/SaveGameBP.HealthLvlChange` (`self.HealthLvlChange`) _output_get)
  (set `/Game/Blueprints/SaveGame/SaveGameBP.SpeedLvlChange` (`self.SpeedLvlChange`) _output_get)
  (set `/Game/Blueprints/SaveGame/SaveGameBP.CoinLvlChange` (`self.CoinLvlChange`) _output_get)
  (set `/Game/Blueprints/SaveGame/SaveGameBP.PlayerAddedHealth` (`self.PlayerAddedHealth`) _output_get)
  (set `/Game/Blueprints/SaveGame/SaveGameBP.PlayerSpeedMultiplayer` (`self.PlayerSpeedMultiplayer`) _output_get)
  (set `/Game/Blueprints/SaveGame/SaveGameBP.AddedCoinsPerCoinBonus` (`self.AddedCoinsPerCoinBonus`) _output_get)
  (set `/Game/Blueprints/SaveGame/SaveGameBP.Shoot infos` (`self.ShootTypeInfos`) _output_get)
  (`GameplayStatics.SaveGameToSlot` (`self.SaveGameObject`) (`self.SaveSlotName`)))

(fn `UpCoinLvl`
  (bind _result (`/Engine/EditorBlueprintResources/StandardMacros.IncrementInt` (`self.CurrentCoinLvl`))
    (:`  `
      (set `self.CurrentCoinLvl` _result))))

(fn `UpHealthLvl`
  (bind _result (`/Engine/EditorBlueprintResources/StandardMacros.IncrementInt` (`self.CurrentHealthLvl`))
    (:`  `
      (set `self.CurrentHealthLvl` _result))))

(fn `UpSpeedLvl`
  (bind _result (`/Engine/EditorBlueprintResources/StandardMacros.IncrementInt` (`self.CurrentSpeedLvl`))
    (:`  `
      (set `self.CurrentSpeedLvl` _result))))