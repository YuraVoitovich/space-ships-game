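; Menu pawn that can be rotated with input axes and can fire several gun presets.
; Holding the right mouse button opens a gate that lets Tick apply axis-driven roll and pitch to the root, scaled by RotationSpeed.
; GunTypeSwitch clears the Shoot component's ShootingInfos, then Simple, Double and Triple presets add their projectile entries and start shooting.
; Fan Cannon and Machine Gun are empty stubs.
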(event `self.ReceiveTick`
  (params (DeltaSeconds :type "Float (single-precision)"))
  (bind _rotationspeed (`self.RotationSpeed`))
  (`/Engine/EditorBlueprintResources/StandardMacros.Gate` true :!label _label
    (:`Exit`
      (`SceneComponent.K2_AddWorldRotation` (`self.DefaultSceneRoot`) (`KismetMathLibrary.MakeRotator` (* _rotationspeed (`self.GetInputAxisKeyValue`)) (* (`self.GetInputAxisKeyValue`) _rotationspeed)) false false))))

(event `Key|RightMouseButton`
  (params (Key :type "Key Structure"))
  (:`Pressed`
    (goto _label :!via `Open`))
  (:`Released`
    (goto _label :!via `Close`)))

(fn `DoubleGun`
  (bind _shoot (`self.Shoot`))
  (bind _shootinginfos (`ShootComponent.ShootingInfos` _shoot))
  (`KismetArrayLibrary.Array_Add` _shootinginfos (make `ShootingManagerInfo` "/Game/Blueprints/Projectiles/BP_ShootProjectile.BP_ShootProjectile_C" (0.0 -20.0 0.0) 0.0 900.0))
  (`KismetArrayLibrary.Array_Add` _shootinginfos (make `ShootingManagerInfo` "/Game/Blueprints/Projectiles/BP_ShootProjectile.BP_ShootProjectile_C" (0.0 20.0 0.0) 0.0 900.0))
  (`ShootComponent.StartShooting` _shoot))

(fn `FanCannon`)

(fn `GunTypeSwitch`
  (params (GunType :type "/Game/Blueprints/Enums/GunTypeEnum Enum" :default "NewEnumerator0"))
  (`KismetArrayLibrary.Array_Clear` (`ShootComponent.ShootingInfos` (`self.Shoot`)))
  (switch `/Game/Blueprints/Enums/GunTypeEnum` GunType
    (:`NewEnumerator0`
      (`self.SimpleGun`))
    (:`NewEnumerator1`
      (`self.DoubleGun`))
    (:`NewEnumerator2`
      (`self.TripleGun`))
    (:`NewEnumerator3`
      (`self.FanCannon`))
    (:`NewEnumerator4`
      (`self.MachineGun`))))

(fn `MachineGun`)

(fn `SimpleGun`
  (bind _shoot (`self.Shoot`))
  (`KismetArrayLibrary.Array_Add` (`ShootComponent.ShootingInfos` _shoot) (make `ShootingManagerInfo` "/Game/Blueprints/Projectiles/BP_ShootProjectile.BP_ShootProjectile_C" (0.0 0.0 0.0) 0.0 900.0))
  (`ShootComponent.StartShooting` _shoot))

(fn `TripleGun`
  (bind _shoot (`self.Shoot`))
  (bind _shootinginfos (`ShootComponent.ShootingInfos` _shoot))
  (`KismetArrayLibrary.Array_Add` _shootinginfos (make `ShootingManagerInfo` "/Game/Blueprints/Projectiles/BP_ShootProjectile.BP_ShootProjectile_C" (0.0 -20.0 0.0) 0.0 900.0 20.0))
  (`KismetArrayLibrary.Array_Add` _shootinginfos (make `ShootingManagerInfo` "/Game/Blueprints/Projectiles/BP_ShootProjectile.BP_ShootProjectile_C" (0.0 20.0 0.0) 0.0 900.0 -20.0))
  (`KismetArrayLibrary.Array_Add` _shootinginfos (make `ShootingManagerInfo` "/Game/Blueprints/Projectiles/BP_ShootProjectile.BP_ShootProjectile_C" (0.0 0.0 0.0) 0.0 900.0))
  (`ShootComponent.StartShooting` _shoot))

(fn `UserConstructionScript`)