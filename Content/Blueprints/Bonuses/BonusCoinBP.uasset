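; BonusCoinBP is a coin bonus actor that carries a coin value and spins in the level.
; On BeginPlay it runs the parent logic, then raises its Coins value by the per-bonus extra stored in MainGameInstance.
; Tick applies a frame-rate-independent local yaw rotation scaled by its rotation speed.
; The file contains no pickup or overlap logic of its own.
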(event `self.ReceiveBeginPlay`
  (`parent.ReceiveBeginPlay`)
  (bind _asmain_game_instance (cast `/Game/Blueprints/GameModes/MainGameInstance` (`GameplayStatics.GetGameInstance`)))
  (set `self.Coins` (+ (`self.Coins`) (`/Game/Blueprints/GameModes/MainGameInstance.AddedCoinsPerCoinBonus` _asmain_game_instance))))

(event `self.ReceiveTick`
  (params (DeltaSeconds :type "Float (single-precision)"))
  (`self.K2_AddActorLocalRotation` (`KismetMathLibrary.MakeRotator` 0.0 0.0 (* DeltaSeconds (`self.RoationSpeed`)))))

(fn `UserConstructionScript`)