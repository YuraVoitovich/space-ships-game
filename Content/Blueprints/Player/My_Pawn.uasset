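; Player pawn that configures its movement speed and weapon from the Main Game Instance when play begins.
; It scales speed by the instance's player multiplier, then GunTypeSwitch sets the shoot delay and branches on the equipped gun type.
; Simple, Double and Triple guns add one to three offset projectile entries to ShootComponent, Triple angling its side shots, then start shooting.
; Fan Cannon and Machine Gun are empty stubs.
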(event `self.ReceiveBeginPlay`
  (`parent.ReceiveBeginPlay`)
  (bind _asmain_game_instance (cast `/Game/Blueprints/GameModes/MainGameInstance` (`GameplayStatics.GetGameInstance`)))
  (set `self.MovementSpeed` (* (`self.MovementSpeed`) (`/Game/Blueprints/GameModes/MainGameInstance.PlayerSpeedMultiplayer` _asmain_game_instance)))
  (bind (_guntypeinfo _guntype) (`/Game/Blueprints/GameModes/MainGameInstance.GetEquptedGun` _asmain_game_instance))
  (`self.GunTypeSwitch` _guntype _guntypeinfo))

(fn `DoubleGun`
  (params (`Shoot info` :type "/Game/Blueprints/Sructure/ShootTypeInfo Structure"))
  (bind _shootcomponent (`self.ShootComponent`))
  (bind _shootinginfos (`ShootComponent.ShootingInfos` _shootcomponent))
  (`KismetArrayLibrary.Array_Add` _shootinginfos (make `ShootingManagerInfo` "/Game/Blueprints/Projectiles/BP_ShootProjectile.BP_ShootProjectile_C" (0.0 -20.0 0.0) `Shoot info_Damage_2_29A2959A4FC03354A9E76B8157FA1F28` `Shoot info_ProjectileSpeed_6_514524CB4BD26B8CC6EEC591A005D50C`))
  (`KismetArrayLibrary.Array_Add` _shootinginfos (make `ShootingManagerInfo` "/Game/Blueprints/Projectiles/BP_ShootProjectile.BP_ShootProjectile_C" (0.0 20.0 0.0) `Shoot info_Damage_2_29A2959A4FC03354A9E76B8157FA1F28` `Shoot info_ProjectileSpeed_6_514524CB4BD26B8CC6EEC591A005D50C`))
  (`ShootComponent.StartShooting` _shootcomponent))

(fn `FanCannon`)

(fn `GunTypeSwitch`
  (params (`Gun Type` :type "/Game/Blueprints/Enums/GunTypeEnum Enum" :default "NewEnumerator0") (ShootingInfo :type "/Game/Blueprints/Sructure/ShootTypeInfo Structure"))
  (set `ShootComponent.ShootDelay` (`.ReloadSpeed_5_18EE95CE4991EB36079440982673F649` (break `/Game/Blueprints/Sructure/ShootTypeInfo` ShootingInfo)) (`self.ShootComponent`))
  (switch `/Game/Blueprints/Enums/GunTypeEnum` `Gun Type`
    (:`NewEnumerator0`
      (`self.Simple Gun` ShootingInfo))
    (:`NewEnumerator1`
      (`self.DoubleGun` ShootingInfo))
    (:`NewEnumerator2`
      (`self.TripleGun` ShootingInfo))
    (:`NewEnumerator3`
      (`self.FanCannon`))
    (:`NewEnumerator4`
      (`self.MachineGun`))))

(fn `MachineGun`)

(fn `Simple Gun`
  (params (ShootInfo :type "/Game/Blueprints/Sructure/ShootTypeInfo Structure"))
  (bind _shootcomponent (`self.ShootComponent`))
  (`KismetArrayLibrary.Array_Add` (`ShootComponent.ShootingInfos` _shootcomponent) (make `ShootingManagerInfo` "/Game/Blueprints/Projectiles/BP_ShootProjectile.BP_ShootProjectile_C" (0.0 0.0 0.0) ShootInfo_Damage_2_29A2959A4FC03354A9E76B8157FA1F28 ShootInfo_ProjectileSpeed_6_514524CB4BD26B8CC6EEC591A005D50C))
  (`ShootComponent.StartShooting` _shootcomponent))

(fn `TripleGun`
  (params (`Shoot Info` :type "/Game/Blueprints/Sructure/ShootTypeInfo Structure"))
  (bind (_damage _reloadspeed _projectilespeed) (break `/Game/Blueprints/Sructure/ShootTypeInfo` `Shoot Info`))
  (bind _shootcomponent (`self.ShootComponent`))
  (bind _shootinginfos (`ShootComponent.ShootingInfos` _shootcomponent))
  (`KismetArrayLibrary.Array_Add` _shootinginfos (make `ShootingManagerInfo` "/Game/Blueprints/Projectiles/BP_ShootProjectile.BP_ShootProjectile_C" (0.0 -20.0 0.0) _damage _projectilespeed 20.0))
  (`KismetArrayLibrary.Array_Add` _shootinginfos (make `ShootingManagerInfo` "/Game/Blueprints/Projectiles/BP_ShootProjectile.BP_ShootProjectile_C" (0.0 20.0 0.0) _damage _projectilespeed -20.0))
  (`KismetArrayLibrary.Array_Add` _shootinginfos (make `ShootingManagerInfo` "/Game/Blueprints/Projectiles/BP_ShootProjectile.BP_ShootProjectile_C" (0.0 0.0 0.0) _damage _projectilespeed))
  (`ShootComponent.StartShooting` _shootcomponent))

(fn `UserConstructionScript`)