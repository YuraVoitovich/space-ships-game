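; BP_EnemyPawn2 is a homing enemy pawn that flies toward the player and destroys itself when out of screen range.
; BeginPlay launches its collision body at the player using physics velocity.
; Each tick adds player-directed steering to that velocity, clamps its speed and aligns rotation to travel direction.
; Once its X is no longer greater than the player's, the steering multiplier is permanently set to a fixed value.
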(event `self.ReceiveTick`
  (params (DeltaSeconds :type "Float (single-precision)"))
  (bind _returnvalue (`GameplayStatics.GetPlayerPawn` 0))
  (bind _returnvalue_x (`KismetMathLibrary.BreakVector` (`self.K2_GetActorLocation`)))
  (bind _pawncollision (`self.PawnCollision`))
  (bind _returnvalue_2 (`self.K2_GetActorLocation` _returnvalue))
  (bind _returnvalue_3 (`self.IsInScreenRange`))
  (if (not _returnvalue_3)
    (`self.K2_DestroyActor`)
    (elif (> _returnvalue_x (.x _returnvalue_2))
      (if (`KismetSystemLibrary.IsValid` _returnvalue)
        (bind _returnvalue_4 (`PrimitiveComponent.GetPhysicsLinearVelocity` (`self.PawnCollision`) "None" :!label _label))
        (`PrimitiveComponent.SetPhysicsLinearVelocity` _pawncollision (`KismetMathLibrary.Vector_ClampSizeMax` (+ _returnvalue_4 (* (`KismetMathLibrary.Normal` (- _returnvalue_2 (`self.K2_GetActorLocation`))) (`self.RotateToPlayerMultiplier`))) 500.0) false "None")
        (bind _returnvalue_5 (`PrimitiveComponent.GetPhysicsLinearVelocity` _pawncollision "None"))
        (`self.K2_SetActorRotation` (`KismetMathLibrary.MakeRotFromXZ` _returnvalue_5 (`KismetMathLibrary.MakeVector` 0.0 0.0 1.0))))
      (else
        (set `self.RotateToPlayerMultiplier` 2.0)
        (goto _label)))))

(event `self.ReceiveBeginPlay`
  (`parent.ReceiveBeginPlay`)
  (`PrimitiveComponent.SetPhysicsLinearVelocity` (`self.PawnCollision`) (* (`KismetMathLibrary.Normal` (`KismetMathLibrary.ProjectVectorOnToPlane` (- (`self.K2_GetActorLocation` (`GameplayStatics.GetPlayerPawn` 0)) (`self.K2_GetActorLocation`)))) 300.0) false "None"))

(fn `UserConstructionScript`)